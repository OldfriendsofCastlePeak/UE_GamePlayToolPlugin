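; Touch gesture component that enables input on its owner, adds the Enhanced Input touch mapping context, and turns one- or two-finger drags into rotate, move and scale calls.
; Each touch tracks per-update deltas, ignoring tiny movements.
; A lone finger rotates.
; With two, one still finger or a truncated zero-degree acos of the unnormalized deltas' dot product means move; otherwise it scales, signed by finger separation change.
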(event `self.ReceiveBeginPlay`
  (bind _returnvalue (`GameplayStatics.GetPlayerController` 0))
  (`|ExecutionSequence`
    (:`then_0`
      (`Actor.EnableInput` (`self.GetOwner`) _returnvalue)
      (`EnhancedInputSubsystemInterface.AddMappingContext` (pcsubsystem `EnhancedInputLocalPlayerSubsystem` _returnvalue) "/CommonGamePlayToolPlugin/Input/Touch_Input_Context.Touch_Input_Context" 0 (struct)))
    (:`then_1`
      (`self.Touch_Initialize`))))

(event `InputTouch`
  (params (Location :type "Vector Structure") (FingerIndex :type "ETouchIndex Enum")))

(event `EnhancedInput|/CommonGamePlayToolPlugin/Input/Touch_InputAction/IA_Touch1_Float2D`
  (params (ActionValue :type "Vector2D Structure") (ElapsedSeconds :type "Float (double-precision)") (TriggeredSeconds :type "Float (double-precision)") (InputAction :type "InputAction Object Reference" :default "/CommonGamePlayToolPlugin/Input/Touch_InputAction/IA_Touch1_Float2D.IA_Touch1_Float2D"))
  ;[1 1 1] Comment
  (:`Triggered`
    (if (not (`self.Touch2Press`))
      (`self.Touch1`))
    (set `self.Touch1Direction` (- ActionValue (`self.Touch1LastLocation`)))
    (set `self.Touch1LastLocation` ActionValue))
  (:`Started`
    (set `self.Touch1Press` true)
    (set `self.Touch1Direction` (0.0 0.0))
    (set `self.Touch1LastLocation` ActionValue))
  (:`Completed`
    (set `self.Touch1Press` false)
    (set `self.Touch1Direction` (0.0 0.0))
    (set `self.Touch1LastLocation` (0.0 0.0))))

(event `EnhancedInput|/CommonGamePlayToolPlugin/Input/Touch_InputAction/IA_Touch2_Float2D`
  (params (ActionValue :type "Vector2D Structure") (ElapsedSeconds :type "Float (double-precision)") (TriggeredSeconds :type "Float (double-precision)") (InputAction :type "InputAction Object Reference" :default "/CommonGamePlayToolPlugin/Input/Touch_InputAction/IA_Touch2_Float2D.IA_Touch2_Float2D"))
  ;[1 1 1] Comment
  (:`Triggered`
    (if (`self.Touch1Press`)
      ;;[1 1 1] 双指操作：Touch1+2将在Touch2中处理
      (`self.Touch1+2` ActionValue)
      (else
        (`self.Touch2`)))
    (set `self.Touch2Direction` (- ActionValue (`self.Touch2LastLocation`)))
    (set `self.Touch2LastLocation` ActionValue))
  (:`Started`
    (set `self.Touch2Press` true)
    (set `self.Touch2LastLocation` ActionValue)
    (set `self.Touch2Direction` (0.0 0.0)))
  (:`Completed`
    (set `self.Touch2Press` false)
    (set `self.Touch2LastLocation` (0.0 0.0))
    (set `self.Touch2Direction` (0.0 0.0))))

(fn `Calculate Touch 2 Direction`
  (params (Touch2Location :type "Vector2D Structure"))
  ;[1 1 1] 计算Touch2的移动方向
  (if (`self.Touch2Press`)
    _))

(fn `Calculate_Touch1_Direction`
  (params (Touch1Location :type "Vector2D Structure"))
  ;[1 1 1] 计算Touch1的移动方向
  (if (`self.Touch1Press`)
    _))

(fn `Touch1`
  (bind _touch1direction (`self.Touch1Direction`))
  ;[1 1 1] 1根手指触碰
  (if (`KismetMathLibrary.IsZero2D` _touch1direction)
    _
    (elif (not (<= (`KismetMathLibrary.Abs` (`KismetMathLibrary.VSize2D` _touch1direction)) 1.0))
      (`self.Touch_Rotation_Action` _touch1direction))))

(fn `Touch1+2`
  (params (New :type "Vector2D Structure"))
  (bind _touch1direction (`self.Touch1Direction`))
  (bind _touch2direction (`self.Touch2Direction`))
  (bind _touch1direction_2 (`self.Touch1Direction`))
  (bind _touch2direction_2 (`self.Touch2Direction`))
  (bind _returnvalue (`KismetMathLibrary.Abs` (`KismetMathLibrary.VSize2D` (- New (`self.Touch2LastLocation`)))))
  (if (`KismetMathLibrary.IsZero2D` (`self.Touch1Direction`))
    (set `self.bTouch1IsZero` true)
    (if (<= (`KismetMathLibrary.Abs` (`KismetMathLibrary.VSize2D` _touch2direction)) 3.0)
      (set `self.Touch2Direction` (0.0 0.0))
      (else
        ;[1 1 1] Touch1移动向量为0,则为双指移动操作传入Touch2移动向量
        (`self.Touch_Move_Action` _touch2direction)))
    (elif (`KismetMathLibrary.IsZero2D` (`self.Touch2Direction`))
      (set `self.bTouch2IsZero` true)
      (if (<= (`KismetMathLibrary.Abs` (`KismetMathLibrary.VSize2D` _touch1direction_2)) 3.0)
        (set `self.Touch1Direction` (0.0 0.0))
        (else
          ;[1 1 1] Touch2移动向量为0,则为双指移动操作传入Touch1移动向量
          (`self.Touch_Move_Action` _touch1direction_2)))
      (elif (== (`KismetMathLibrary.FTrunc` (`KismetMathLibrary.DegAcos` (`KismetMathLibrary.DotProduct2D` (`self.Touch1Direction`) (`self.Touch2Direction`)))) 0)
        (if (<= (`KismetMathLibrary.Abs` (`KismetMathLibrary.VSize2D` _touch1direction)) 1.0)
          (if (not (<= (`KismetMathLibrary.Abs` (`KismetMathLibrary.VSize2D` _touch2direction_2)) 1.0))
            (`self.Touch_Move_Action` _touch2direction_2))
          (else
            (`self.Touch_Move_Action` _touch1direction)))
        (elif (not (<= _returnvalue 1.0))
          (`self.Touch_Scale_Action` (* (`KismetMathLibrary.SelectFloat` 1.0 -1.0 (> (`KismetMathLibrary.VSize2D` (- New (`self.Touch1LastLocation`))) (`KismetMathLibrary.VSize2D` (- (`self.Touch2LastLocation`) (`self.Touch1LastLocation`))))) _returnvalue)))))))

(fn `Touch2`
  (bind _touch2direction (`self.Touch2Direction`))
  ;[1 1 1] 1根手指触碰
  (if (`KismetMathLibrary.IsZero2D` _touch2direction)
    _
    (elif (not (<= (`KismetMathLibrary.Abs` (`KismetMathLibrary.VSize2D` _touch2direction)) 1.0))
      (`self.Touch_Rotation_Action` _touch2direction))))