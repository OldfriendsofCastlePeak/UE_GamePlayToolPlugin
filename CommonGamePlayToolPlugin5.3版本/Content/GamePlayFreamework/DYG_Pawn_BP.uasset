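; DYG_Pawn_BP is a mouse-driven viewer Pawn that pans on left drag, rotates on right drag and wheel-zooms.
; It swaps between a normal camera and a spring-arm orbit camera by pitch range, deriving arm length from height and pitch sine to preserve the viewpoint.
; Pan speed scales with arm length within XY bounds, and a timeline smooths zoom.
; Events handle view placement, camera blends with re-possession, and attachment; idle auto-rotation is unwired.
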(event `self.ReceiveBeginPlay`
  ;[0.6225 0.6817 1] 执行开始，注册输入上下文
  (`self.EnableInput` (`GameplayStatics.GetPlayerController` 0))
  (`EnhancedInputSubsystemInterface.AddMappingContext` (pcsubsystem `EnhancedInputLocalPlayerSubsystem` (`GameplayStatics.GetPlayerController` 0)) "/CommonGamePlayToolPlugin/Input/Game_Input_Context.Game_Input_Context" 0 (struct)))

(event `self.ReceiveTick`
  (params (DeltaSeconds :type "Float (single-precision)"))
  ;[1 1 1] Comment
)

(event `Auto_Rotator_Rest_Event`
  ;[1 1 1] Comment
)

(event `Key|LeftMouseButton`
  (params (Key :type "Key Structure"))
  ;[0.5948 0.6891 1] 鼠标左右按键按下与松开
  (:`Pressed`
    (set `self.L_Mouse_Pressed` true)
    (`self.Auto_Rotator_Rest_Event` :!label _label))
  (:`Released`
    (set `self.L_Mouse_Pressed` false)
    (goto _label)))

(event `Key|RightMouseButton`
  (params (Key :type "Key Structure"))
  ;[0.5948 0.6891 1] 鼠标左右按键按下与松开
  (:`Pressed`
    (set `self.R_Mouse_Pressed` true)
    (goto _label))
  (:`Released`
    (set `self.R_Mouse_Pressed` false)
    (goto _label)))

(event `EnhancedInput|/CommonGamePlayToolPlugin/Input/Input_Float2D/IA_Float2D_Mouse`
  (params (ActionValue :type "Vector2D Structure") (ElapsedSeconds :type "Float (double-precision)") (TriggeredSeconds :type "Float (double-precision)") (InputAction :type "InputAction Object Reference" :default "/CommonGamePlayToolPlugin/Input/Input_Float2D/IA_Float2D_Mouse.IA_Float2D_Mouse"))
  ;[0.6892 0.7388 1] 鼠标移动——控制Pawn移动、旋转
  (:`Triggered`
    (if (`self.CanMove`)
      (`self.Active_Camera`
        (:`Normal_Camera_Active`
          (`self.Mouse_Press_State`
            (:`L_Press`
              (if (`KismetMathLibrary.InRange_FloatFloat` (.pitch (`self.K2_GetActorRotation`)) (`self.View_Pitch_Min_Value`) (`self.View_Pitch_Max_Value`))
                (`self.NormalCamera_To_SpringArmCamera`)
                (else
                  (`self.Normal_Camear_Pawn_Move` ActionValue))))
            (:`R_Press`
              (`self.Normal_Camear_Pawn_Rotator` ActionValue)))
          (`self.Auto_Rotator_Rest_Event` :!label _label_2))
        (:`Spring_Arm_Camera_Active`
          (if (`KismetMathLibrary.InRange_FloatFloat` (.pitch (`self.K2_GetActorRotation`)) (`self.View_Pitch_Min_Value`) (`self.View_Pitch_Max_Value`))
            (`self.Mouse_Press_State`
              (:`L_Press`
                (`self.SpringArm_Move_Pawn` ActionValue)
                (goto _label_2))
              (:`R_Press`
                (`self.SpringArm_Rotator_Pawn` ActionValue)
                (goto _label_2)))
            (else
              (`self.SpringArmCamera_To_NormalCamera`)
              (goto _label_2))))
        (:`None_Active`
          (`KismetSystemLibrary.PrintString` "Erro：Pawn上没有激活的Camera"))))))

(event `EnhancedInput|/CommonGamePlayToolPlugin/Input/Input_Float1D/IA_Float1D_MouseWheel`
  (params (ActionValue :type "Float (double-precision)") (ElapsedSeconds :type "Float (double-precision)") (TriggeredSeconds :type "Float (double-precision)") (InputAction :type "InputAction Object Reference" :default "/CommonGamePlayToolPlugin/Input/Input_Float1D/IA_Float1D_MouseWheel.IA_Float1D_MouseWheel"))
  (bind _targetarmlength (`SpringArmComponent.TargetArmLength` (`self.SpringArm`)))
  (bind _returnvalue (* _targetarmlength 0.2))
  ;[0.6389 0.6583 1] 鼠标滚轮滑动——控制Pawn的Spring Arm长度
  (:`Triggered`
    (if (`self.CanMove`)
      (if (`KismetMathLibrary.InRange_FloatFloat` (.pitch (`self.K2_GetActorRotation`)) (`self.View_Pitch_Min_Value`) (`self.View_Pitch_Max_Value`))
        (`self.NormalCamera_To_SpringArmCamera`)
        (set `self.Cur_ArmLength` (`KismetMathLibrary.FTrunc` _targetarmlength))
        (set `self.Tar_ArmLength` (`KismetMathLibrary.FTrunc` (`KismetMathLibrary.FClamp` (- _targetarmlength (* ActionValue (`KismetMathLibrary.FClamp` _returnvalue 1000.0 _returnvalue))) 0.0 2000000.0)))
        (`self.Auto_Rotator_Rest_Event`)
        (`Timeline|SpringArm_TimeLine` :!via `PlayFromStart`
          (:`Update`
            (set `SpringArmComponent.TargetArmLength` (`KismetMathLibrary.FInterpTo` (`SpringArmComponent.TargetArmLength` (`self.SpringArm`)) (`KismetMathLibrary.Conv_IntToDouble` (`self.Tar_ArmLength`)) (`GameplayStatics.GetWorldDeltaSeconds`) 2.0) (`self.SpringArm`))))
        (else
          (`KismetSystemLibrary.PrintString` "角度Pitch超出范围，无法缩放视角"))))))

(event `Set_Camera_View_Location`
  (params (View_Actor :type "Actor Object Reference"))
  ;[0.295 0.5986 1] 直接设置相机应处于的位置——普通相机的相对位置归零，直接设置Pawn的位置和方向也就是普通相机的位置和角度
  (`self.SpringArmCamera_To_NormalCamera`)
  (`self.K2_SetActorLocation` (`self.K2_GetActorLocation` View_Actor))
  (`self.K2_SetActorRotation` (`KismetMathLibrary.MakeRotator` (.roll (`self.K2_GetActorRotation` View_Actor)) (.pitch (`self.K2_GetActorRotation` View_Actor)) (.yaw (`self.K2_GetActorRotation` View_Actor)))))

(event `Blend_View_To_Camera_Actor`
  (params (Camera_Name :type Name))
  ;[0.6012 0.6727 1] 混合视口到Camera_Actor
  ;;[1 1 1] 储存一下，用于在视口混合完毕之后对特定相机混合进行处理
  (set `self.CurrentBlendCameraName` Camera_Name)
  (`/Engine/EditorBlueprintResources/StandardMacros.IsValid` null
    (:`Is Valid`
      ;;[1 1 1] 进行视口混合
      (bind _ascamera_actor (cast `CameraActor` null)
        (:`then`
          (bind _cameracomponent (`CameraActor.CameraComponent` _ascamera_actor))
          (set `CameraComponent.bConstrainAspectRatio` false _cameracomponent)
          (set `CameraComponent.bLockToHmd` false _cameracomponent))
        (:`CastFailed`
          _))
      (`KismetSystemLibrary.PrintString` "开始进行视角混合")
      ;;[1 1 1] 表示正在进行视角混合
      (set `self.Is_Playing_View_Blend` true)
      ;;[1 1 1] 进行视口混合时，设定视口最终应该处于的位置，以避免视口混合完时重新控制Pawn时位置不一致
      (`PlayerController.SetViewTargetWithBlend` (`GameplayStatics.GetPlayerController` 0) null 1.0 "VTBlend_Linear" 1.0 true)
      (`self.Set_Camera_View_Location` null)
      (set `self.TemTimer` 0.0)
      (`self.Auto_Rotator_Rest_Event`)
      (if (>= (`self.TemTimer`) 1.0) :!label _label_3
        (`self.View_Blend_Complete_Custom_Event`)
        (else
          (`KismetSystemLibrary.Delay` 0.2)
          (set `self.TemTimer` (+ (`self.TemTimer`) 0.2))
          (goto _label_3))))
    (:`Is Not Valid`
      (`KismetSystemLibrary.PrintString` (`KismetStringLibrary.Concat_StrStr` "未找到对应的Actor:" (`KismetStringLibrary.Conv_NameToString` (`self.CurrentBlendCameraName`)))))))

(event `Pawn_Attach_To_Actor`
  (params (NewParam :type "SceneComponent Object Reference"))
  (`self.SpringArmCamera_To_NormalCamera`)
  (`self.K2_AttachToComponent` NewParam "None" "SnapToTarget" "SnapToTarget" "KeepRelative"))

(event `Pawn_Deattach`
  (`self.K2_DetachFromActor` self "KeepWorld" "KeepWorld" "KeepWorld"))

(event `View_Blend_Complete_Custom_Event`
  ;[0.7185 0.577 1] 视口混合完毕,重新控制Pawn
  (`Controller.Possess` (`GameplayStatics.GetPlayerController` 0) self))

(fn `Normal_Camear_Pawn_Move`
  (params (Input :type "Vector2D Structure"))
  (bind (_min_move_location_x _min_move_location_y) (`KismetMathLibrary.BreakVector2D` (`self.Min_Move_Location`)))
  (bind (_max_move_location_x _max_move_location_y) (`KismetMathLibrary.BreakVector2D` (`self.Max_Move_Location`)))
  (bind _returnvalue (`PlayerCameraManager.GetCameraRotation` (`GameplayStatics.GetPlayerCameraManager` 0)))
  (bind (_returnvalue_x _returnvalue_y) (`KismetMathLibrary.BreakVector` (`KismetMathLibrary.GetForwardVector` _returnvalue)))
  (bind (_returnvalue_x_2 _returnvalue_y_2) (`KismetMathLibrary.BreakVector` (`KismetMathLibrary.GetRightVector` _returnvalue)))
  (bind _returnvalue_2 (* (`SpringArmComponent.TargetArmLength` (`self.SpringArm`)) 0.005))
  (bind _returnvalue_3 (`KismetMathLibrary.FClamp` _returnvalue_2 50.0 _returnvalue_2))
  (`self.K2_SetActorLocation` (`KismetMathLibrary.MakeVector` (`KismetMathLibrary.FClamp` (.x (+ (* (* Input_X -1.0 _returnvalue_3) (`KismetMathLibrary.Normal` (`KismetMathLibrary.MakeVector` _returnvalue_x_2 _returnvalue_y_2))) (* (* Input_Y -1.0 _returnvalue_3) (`KismetMathLibrary.Normal` (`KismetMathLibrary.MakeVector` _returnvalue_x _returnvalue_y))) (`self.K2_GetActorLocation`))) _min_move_location_x _min_move_location_y) (`KismetMathLibrary.FClamp` (.y (+ (* (* Input_X -1.0 _returnvalue_3) (`KismetMathLibrary.Normal` (`KismetMathLibrary.MakeVector` _returnvalue_x_2 _returnvalue_y_2))) (* (* Input_Y -1.0 _returnvalue_3) (`KismetMathLibrary.Normal` (`KismetMathLibrary.MakeVector` _returnvalue_x _returnvalue_y))) (`self.K2_GetActorLocation`))) _max_move_location_x _max_move_location_y) (.z (+ (* (* Input_X -1.0 _returnvalue_3) (`KismetMathLibrary.Normal` (`KismetMathLibrary.MakeVector` _returnvalue_x_2 _returnvalue_y_2))) (* (* Input_Y -1.0 _returnvalue_3) (`KismetMathLibrary.Normal` (`KismetMathLibrary.MakeVector` _returnvalue_x _returnvalue_y))) (`self.K2_GetActorLocation`))))))

(fn `Normal_Camear_Pawn_Rotator`
  (params (Input :type "Vector2D Structure"))
  (`self.K2_SetActorRotation` (`KismetMathLibrary.MakeRotator` (.roll (`self.K2_GetActorRotation`)) (`KismetMathLibrary.FClamp` (+ (.pitch (`self.K2_GetActorRotation`)) (* Input_Y 1.0 0.8)) -89.0 89.0) (+ (.yaw (`self.K2_GetActorRotation`)) (* Input_X 1.0 0.8)))))

(fn `NormalCamera_To_SpringArmCamera`
  (locals (Current_Camera_Rot :type "Rotator Structure" :default (struct)) (Current_Camera_Loc :type "Vector Structure" :default (0.0 0.0 0.0)))
  (bind (_current_camera_loc_x _current_camera_loc_y _current_camera_loc_z) (`KismetMathLibrary.BreakVector` (`local.Current_Camera_Loc`)))
  (bind (_current_camera_loc_x_2 _current_camera_loc_y_2 _current_camera_loc_z_2) (`KismetMathLibrary.BreakVector` (`local.Current_Camera_Loc`)))
  ;[1 1 1] 检查弹簧臂相机是否激活
  (if (`ActorComponent.IsActive` (`self.SpringArm_Camera`))
    ;[1 1 1] 检查弹簧臂相机已经处于激活状态，开启相机Lag
    (set `SpringArmComponent.bEnableCameraLag` true (`self.SpringArm`))
    (else
      ;[1 1 1] 获取当前Actor角度、位置（也就是Normal_Camera的位置、角度）。便于后面进行计算
      (set `local.Current_Camera_Rot` (`self.K2_GetActorRotation`))
      (set `local.Current_Camera_Loc` (`self.K2_GetActorLocation`))
      ;[1 1 1] 检查当前位置的Z轴高度，是否处于限定范围
      (if (>= _current_camera_loc_z (`self.Min_Z_Value`))
        ;[1 1 1] 计算最终Pawn的位置，并计算弹簧臂应该设定的长度
        (bind _output_get (set `SpringArmComponent.TargetArmLength` (/ (- _current_camera_loc_z_2 (`self.Min_Z_Value`)) (`KismetMathLibrary.Abs` (`KismetMathLibrary.DegSin` (.pitch (`local.Current_Camera_Rot`))))) (`self.SpringArm`)))
        (`self.K2_SetActorLocation` (+ (`local.Current_Camera_Loc`) (* (`KismetMathLibrary.GetForwardVector` (`local.Current_Camera_Rot`)) _output_get)))
        ;[1 1 1] 一切条件满足，激活弹簧臂相机、灭活普通相机
        (`ActorComponent.SetActive` (`self.SpringArm_Camera`) true false)
        (`ActorComponent.SetActive` (`self.Normal_Camera`) false false)
        (else
          (`KismetSystemLibrary.PrintString` "Erro：Z轴位置错误，超出限定范围，，无法切换相机"))))))

(fn `SpringArm_Move_Pawn`
  (params (InputAction :type "Vector2D Structure"))
  (bind (_min_move_location_x _min_move_location_y) (`KismetMathLibrary.BreakVector2D` (`self.Min_Move_Location`)))
  (bind (_max_move_location_x _max_move_location_y) (`KismetMathLibrary.BreakVector2D` (`self.Max_Move_Location`)))
  (bind _returnvalue (`PlayerCameraManager.GetCameraRotation` (`GameplayStatics.GetPlayerCameraManager` 0)))
  (bind (_returnvalue_x _returnvalue_y) (`KismetMathLibrary.BreakVector` (`KismetMathLibrary.GetForwardVector` _returnvalue)))
  (bind (_returnvalue_x_2 _returnvalue_y_2) (`KismetMathLibrary.BreakVector` (`KismetMathLibrary.GetRightVector` _returnvalue)))
  (bind _returnvalue_2 (* (`SpringArmComponent.TargetArmLength` (`self.SpringArm`)) 0.008))
  (bind _returnvalue_3 (`KismetMathLibrary.FClamp` _returnvalue_2 50.0 _returnvalue_2))
  ;[1 1 1] 在原本的位置上加上要移动的位置
  (`self.K2_SetActorLocation` (`KismetMathLibrary.MakeVector` (`KismetMathLibrary.FClamp` (.x (+ (* (* InputAction_X -1.0 _returnvalue_3) (`KismetMathLibrary.Normal` (`KismetMathLibrary.MakeVector` _returnvalue_x_2 _returnvalue_y_2))) (* (* InputAction_Y -1.0 _returnvalue_3) (`KismetMathLibrary.Normal` (`KismetMathLibrary.MakeVector` _returnvalue_x _returnvalue_y))) (`self.K2_GetActorLocation`))) _min_move_location_x _min_move_location_y) (`KismetMathLibrary.FClamp` (.y (+ (* (* InputAction_X -1.0 _returnvalue_3) (`KismetMathLibrary.Normal` (`KismetMathLibrary.MakeVector` _returnvalue_x_2 _returnvalue_y_2))) (* (* InputAction_Y -1.0 _returnvalue_3) (`KismetMathLibrary.Normal` (`KismetMathLibrary.MakeVector` _returnvalue_x _returnvalue_y))) (`self.K2_GetActorLocation`))) _max_move_location_x _max_move_location_y) (.z (+ (* (* InputAction_X -1.0 _returnvalue_3) (`KismetMathLibrary.Normal` (`KismetMathLibrary.MakeVector` _returnvalue_x_2 _returnvalue_y_2))) (* (* InputAction_Y -1.0 _returnvalue_3) (`KismetMathLibrary.Normal` (`KismetMathLibrary.MakeVector` _returnvalue_x _returnvalue_y))) (`self.K2_GetActorLocation`))))))

(fn `SpringArm_Rotator_Pawn`
  (params (InputAction :type "Vector2D Structure"))
  (`self.K2_SetActorRotation` (`KismetMathLibrary.MakeRotator` (.roll (`self.K2_GetActorRotation`)) (`KismetMathLibrary.FClamp` (+ (.pitch (`self.K2_GetActorRotation`)) (* InputAction_Y 1.0 1.0)) (`self.View_Pitch_Min_Value`) (`self.View_Pitch_Max_Value`)) (+ (.yaw (`self.K2_GetActorRotation`)) (* InputAction_X 1.0 1.0)))))

(fn `SpringArmCamera_To_NormalCamera`
  (bind _springarm (`self.SpringArm`))
  ;[1 1 1] 检查普通的相机是否激活，激活则不需要操作。只有从弹簧臂相机到普通相机才需要。
  (if (not (`ActorComponent.IsActive` (`self.Normal_Camera`)))
    ;[1 1 1] 归零普通相机的相对旋转，只有这样普通相机使用的才是Pawn的角度
    (`SceneComponent.K2_SetRelativeTransform` (`self.Normal_Camera`) (`KismetMathLibrary.MakeTransform` (0.0 0.0 0.0)) false false)
    ;[1 1 1] 激活普通相机、灭活弹簧臂相机
    (`ActorComponent.SetActive` (`self.Normal_Camera`) true false)
    (`ActorComponent.SetActive` (`self.SpringArm_Camera`) false false)
    ;[1 1 1] 归零弹簧比的长度和取消相机Lag
    (set `SpringArmComponent.TargetArmLength` 0.0 _springarm)
    (set `SpringArmComponent.bEnableCameraLag` false _springarm)))

(fn `UserConstructionScript`)