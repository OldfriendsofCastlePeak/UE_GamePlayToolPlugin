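; Common_Pawn_BP is a player pawn with a mouse-controlled spring arm camera.
; On BeginPlay it shows the cursor and sets Game and UI input mode.
; Mouse XY and wheel input feed inherited camera input handlers, while left and right buttons set the move and rotate action states.
; Leftover nodes for UI creation, camera switching, pitch range and collision testing are unconnected and never run.
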(event `self.ReceiveBeginPlay`
  (bind _returnvalue (`GameplayStatics.GetPlayerController` 0))
  (`parent.ReceiveBeginPlay`)
  (`WidgetBlueprintLibrary.SetInputMode_GameAndUIEx` _returnvalue null)
  (set `PlayerController.bShowMouseCursor` true _returnvalue))

(event `self.MouseInput.MouseXYInput`
  (params (Value :type "Vector2D Structure"))
  (`self.ReceiveFVector2DInputEvent` Value))

(event `self.MouseInput.MouseLeftButtonInput`
  (params (Value :type Boolean))
  (set `self.bMove_Action_Type` Value))

(event `self.MouseInput.MouseRightButtonInput`
  (params (Value :type Boolean))
  (set `self.bRotate_Action_Type` Value))

(event `self.MouseInput.MouseWheelInput`
  (params (Value :type "Float (single-precision)"))
  (`self.SpringArm_Camera_Receive_Float_Input_Event` Value))

(fn `UserConstructionScript`
  (`parent.UserConstructionScript`))