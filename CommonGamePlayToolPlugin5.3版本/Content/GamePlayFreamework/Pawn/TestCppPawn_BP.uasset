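; Test pawn for touch-driven rotation with a normal camera and a spring arm camera, built on inherited camera helpers.
; BeginPlay sets the starting rotation, Game-and-UI input with visible cursor, and the main UI widget.
; When movement is allowed, touch drags rotate via the active camera, switching from normal to spring arm within a pitch range and resetting the auto-rotate timer.
; Input values and sequence playback start/finish print as debug text.
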(event `self.SetupPlayerInputComponent_Internal`
  (`TouchBaseComponent.RegisterTouchInput` (`self.SingleTouch`)))

(event `self.ReceiveBeginPlay`
  (bind _returnvalue (`GameplayStatics.GetPlayerController` 0))
  (`parent.ReceiveBeginPlay`)
  (`self.K2_SetActorRotation` (struct :`Pitch` -45.0))
  (`WidgetBlueprintLibrary.SetInputMode_GameAndUIEx` _returnvalue null "DoNotLock" false)
  (set `PlayerController.bShowMouseCursor` true _returnvalue)
  (bind _returnvalue_2 (`|CreateWidget` "/CommonGamePlayToolPlugin/UI/Touch/Main_UI_WBP.Main_UI_WBP_C"))
  (`UserWidget.AddToViewport` _returnvalue_2 0)
  (set `self.NewVar` (`self.GetInstigatorController`)))

(event `self.ViewBlendComponent.OnEndViewBlend`)

(event `self.PlaySequenceTool.FinshPlaySequence`
  (`KismetSystemLibrary.PrintString` "播放完毕"))

(event `self.PlaySequenceTool.StartPlaySequenceEvent`
  (`KismetSystemLibrary.PrintString` "开始播放"))

(event `self.SingleTouch.On_Touch_Moved`
  (params (Location :type "Vector Structure"))
  (bind _returnvalue (`KismetMathLibrary.Conv_VectorToVector2D` Location))
  (bind (_returnvalue_roll _returnvalue_pitch) (`KismetMathLibrary.BreakRotator` (`self.K2_GetActorRotation`)))
  (bind (_normal_camera_to_springarm_camera_rotate_pitch_range_x _normal_camera_to_springarm_camera_rotate_pitch_range_y) (`KismetMathLibrary.BreakVector2D` (`self.Normal_Camera_To_SpringArm_Camera_Rotate_Pitch_Range`)))
  (if (`self.bCan_Move`)
    (`self.GetCurrentActiveCamera`
      (:`Only_SpringArm_Camera_Active`
        (bind _returnvalue_2 (`self.Normal_Camera_To_SpringArm_Camera`))
        (if _returnvalue_2
          (`self.SpringArm_Camera_Rotate_Pawn` _returnvalue)
          (`self.Reset_Auto_Rotate_Total_Time`)))
      (:`Only_Normal_Camera_Active`
        (if (and (>= _returnvalue_pitch _normal_camera_to_springarm_camera_rotate_pitch_range_x) (<= _returnvalue_pitch _normal_camera_to_springarm_camera_rotate_pitch_range_y))
          (`self.Normal_Camera_To_SpringArm_Camera`)
          (else
            (`self.Normal_Camera_Rotate_Pawn` _returnvalue)
            (`self.Reset_Auto_Rotate_Total_Time`)))))))

(event `self.ReceiveTick`
  (params (DeltaSeconds :type "Float (single-precision)"))
  (`KismetSystemLibrary.PrintString` (`KismetStringLibrary.Conv_IntToString` (`self.GetAllInput`)) true true (struct :`G` 0.66 :`B` 1.0 :`A` 1.0) 0.0))

(event `self.KeyboardInput.Keyboard_A_Input`
  (params (Value :type "Float (single-precision)"))
  (`KismetSystemLibrary.PrintString` (`KismetStringLibrary.Concat_StrStr` "A的值为：" (`KismetStringLibrary.Conv_DoubleToString` Value))))

(fn `UserConstructionScript`
  (`parent.UserConstructionScript`))